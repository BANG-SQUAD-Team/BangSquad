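; BP_Demon1 is a demon minion with a modular skeletal mesh whose stones, basket and stone weapon can be toggled.
; The construction script makes the six stone meshes and the basket follow the main Mesh's animation as leader pose.
; It then sets each piece's visibility from boolean variables, with the Niagara effect sharing the basket's flag.
; The event graph holds no gameplay logic.
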(event `self.ReceiveBeginPlay`)

(fn `UserConstructionScript`
  (`SkinnedMeshComponent.SetLeaderPoseComponent` (`self.Stone5`) (`self.Mesh`) true false)
  (`SkinnedMeshComponent.SetLeaderPoseComponent` (`self.Stone4`) (`self.Mesh`) true false)
  (`SkinnedMeshComponent.SetLeaderPoseComponent` (`self.Stone3`) (`self.Mesh`) true false)
  (`SkinnedMeshComponent.SetLeaderPoseComponent` (`self.Stone2`) (`self.Mesh`) true false)
  (`SkinnedMeshComponent.SetLeaderPoseComponent` (`self.Stone1`) (`self.Mesh`) true false)
  (`SkinnedMeshComponent.SetLeaderPoseComponent` (`self.SKM_Basket`) (`self.Mesh`) true false)
  (`SkinnedMeshComponent.SetLeaderPoseComponent` (`self.Stone6`) (`self.Mesh`) true false)
  (`|ExecutionSequence`
    (:`then_0`
      (`SceneComponent.SetVisibility` (`self.Stone5`) (`self.Stone5_Visibility`) false))
    (:`then_1`
      (`SceneComponent.SetVisibility` (`self.Stone6`) (`self.Stone6_Visibility`) false))
    (:`then_2`
      (`SceneComponent.SetVisibility` (`self.SM_Stone_Weapon`) (`self.Weapon_Visibility`) false))
    (:`then_3`
      (`SceneComponent.SetVisibility` (`self.SKM_Basket`) (`self.Basket_Visibility`) false)
      (`SceneComponent.SetVisibility` (`self.Niagara`) (`self.Basket_Visibility`) false))
    (:`then_4`
      (`SceneComponent.SetVisibility` (`self.Stone1`) (`self.Stone1_Visibility`) false))
    (:`then_5`
      (`SceneComponent.SetVisibility` (`self.Stone2`) (`self.Stone2_Visibility`) false))
    (:`then_6`
      (`SceneComponent.SetVisibility` (`self.Stone3`) (`self.Stone3_Visibility`) false))
    (:`then_7`
      (`SceneComponent.SetVisibility` (`self.Stone4`) (`self.Stone4_Visibility`) false))))