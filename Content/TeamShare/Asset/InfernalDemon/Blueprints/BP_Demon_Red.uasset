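; BP_Demon_Red is a modular demon Blueprint with optional wings, wing flame and armor pieces.
; The construction script makes each skeletal mesh part follow the main Mesh through Set Leader Pose Component, so they animate with the body.
; It then sets each part's visibility from its own variable, allowing different looks to be configured.
; The event graph holds only empty default events, so there is no gameplay logic.
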(event `self.ReceiveBeginPlay`)

(fn `UserConstructionScript`
  (`SkinnedMeshComponent.SetLeaderPoseComponent` (`self.SKM_Hands_Armor`) (`self.Mesh`) true false)
  (`SkinnedMeshComponent.SetLeaderPoseComponent` (`self.SKM_Legs_Armor`) (`self.Mesh`) true false)
  (`SkinnedMeshComponent.SetLeaderPoseComponent` (`self.SKM_Shoulder_Pads`) (`self.Mesh`) true false)
  (`SkinnedMeshComponent.SetLeaderPoseComponent` (`self.SKM_Spine_Armor`) (`self.Mesh`) true false)
  (`SkinnedMeshComponent.SetLeaderPoseComponent` (`self.SKM_Thigh_Armor`) (`self.Mesh`) true false)
  (`SkinnedMeshComponent.SetLeaderPoseComponent` (`self.SKM_Wing_Part`) (`self.Mesh`) true false)
  (`SkinnedMeshComponent.SetLeaderPoseComponent` (`self.SKM_Wings`) (`self.Mesh`) true false)
  (`SkinnedMeshComponent.SetLeaderPoseComponent` (`self.SKM_Chest_Armor`) (`self.Mesh`) true false)
  (`|ExecutionSequence`
    (:`then_0`
      (`SceneComponent.SetVisibility` (`self.SKM_Wings`) (`self.Wings_Visibility`) false))
    (:`then_1`
      (`SceneComponent.SetVisibility` (`self.SKM_Wing_Part`) (`self.Wings_Flame_Visibility`) false))
    (:`then_2`
      (`SceneComponent.SetVisibility` (`self.SKM_Shoulder_Pads`) (`self.Shoulder_Pads_Visibility`) false))
    (:`then_3`
      (`SceneComponent.SetVisibility` (`self.SKM_Chest_Armor`) (`self.Chest_Armor_Visibility`) false))
    (:`then_4`
      (`SceneComponent.SetVisibility` (`self.SKM_Hands_Armor`) (`self.Hands_Armor_Visibility`) false))
    (:`then_5`
      (`SceneComponent.SetVisibility` (`self.SKM_Legs_Armor`) (`self.Legs_Armor_Visibility`) false))
    (:`then_6`
      (`SceneComponent.SetVisibility` (`self.SKM_Spine_Armor`) (`self.Spine_Armor_Visibility`) false))
    (:`then_7`
      (`SceneComponent.SetVisibility` (`self.SKM_Thigh_Armor`) (`self.Thigh_Armor_Visibility`) false))))